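; BP_Player_COM is the computer-controlled paddle in a Pong-style game, held at a fixed X position and moving along Z.
; Each tick it reads the ball reference from BP_GM_Paddle and follows the ball's height only while the ball moves toward negative X, otherwise holding still.
; Without a valid ball it returns to Z zero, using constant-speed interpolation for all movement.
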(event `self.ReceiveTick`
  (params (DeltaSeconds :type "Float (single-precision)"))
  (bind _ref_ball (`self.Ref_Ball`))
  (bind _returnvalue_x (`KismetMathLibrary.BreakVector` (`self.GetVelocity` _ref_ball)))
  (bind (_returnvalue_x_2 _returnvalue_y _returnvalue_z) (`KismetMathLibrary.BreakVector` (`self.K2_GetActorLocation` _ref_ball)))
  (`parent.ReceiveTick` DeltaSeconds)
  (bind _asbp_gm_paddle (cast `/Game/Blueprints/BP_GM_Paddle` (`GameplayStatics.GetGameMode`)))
  (bind _output_get (set `self.Ref_Ball` (`/Game/Blueprints/BP_GM_Paddle.Ref_Ball` _asbp_gm_paddle)))
  (`/Engine/EditorBlueprintResources/StandardMacros.IsValid` _output_get
    (:`Is Valid`
      (if (< _returnvalue_x 0.0)
        (`self.K2_SetActorLocation` (`KismetMathLibrary.VInterpTo_Constant` (`self.K2_GetActorLocation`) (`KismetMathLibrary.MakeVector` -1440.0 0.0 _returnvalue_z) (`GameplayStatics.GetWorldDeltaSeconds`) (`self.Speed`)))))
    (:`Is Not Valid`
      (`self.K2_SetActorLocation` (`KismetMathLibrary.VInterpTo_Constant` (`self.K2_GetActorLocation`) (`KismetMathLibrary.MakeVector` -1440.0) (`GameplayStatics.GetWorldDeltaSeconds`) (`self.Speed`))))))

(fn `UserConstructionScript`
  (`parent.UserConstructionScript`))