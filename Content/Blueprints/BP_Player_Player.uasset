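; Player Blueprint that moves itself along the world Z axis from player input.
; The MoveFordward axis event adds a world offset on Z each frame, scaled by the axis value, the Speed variable and delta time, so despite its name the movement is vertical.
; BeginPlay, overlap and Tick are disabled stubs, and the construction script only calls its parent.
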(event `InputAxis|MoveFordward`
  (params (AxisValue :type "Float (single-precision)"))
  (`self.K2_AddActorWorldOffset` (`KismetMathLibrary.MakeVector` 0.0 0.0 (* AxisValue (`GameplayStatics.GetWorldDeltaSeconds`) (`self.Speed`)))))

(fn `UserConstructionScript`
  (`parent.UserConstructionScript`))